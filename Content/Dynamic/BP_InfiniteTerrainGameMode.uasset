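; Game mode for an infinite terrain game that spawns the starting run of tiles and keeps the score.
; On BeginPlay it populates a pool of nav mesh bounds volumes, then spawns tiles in a loop, handing each the pool.
; Each new tile's attach location becomes the next spawn transform, chaining tiles end to end.
; TileBeaten increments the score, which GetScore returns.
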(event EventBeginPlay
  (Class|InfiniteTerrainGameMode|PopulateBoundsVolumePool)
  (for _index (range 0 3)
    (CallFunction|SpawnTile)))

(fn ConstructionScript)

(fn SpawnTile
  ;[1 1 1] Spawn a Tile_BP and store its Arrow transform in our variable for the next iteration of the loop.
  (bind _returnvalue (Game|SpawnActorfromClass "/Game/Dynamic/Terrain/BP_Tile.BP_Tile_C" (Variables|Default|GetNext%20Tile%20Transform) "Undefined" 0 0))
  (Class|Tile|SetActorPool _returnvalue (Variables|Default|GetNavMeshBoundsVolumePool))
  (bind _attach_transform (Default|GetAttachLocation _returnvalue))
  (Variables|Default|SetNext%20Tile%20Transform _attach_transform))

(fn TileBeaten
  (Math|Integer|IncrementInt (Variables|Default|GetScore)))

(fn GetScore
  (return (Variables|Default|GetScore)))