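; AI controller for guard NPCs that detects non-enemy actors and attacks whichever actor it focuses on.
; BeginPlay sets up the guard blackboard and runs the guard behavior tree.
; Perception updates store sensed actors lacking the Enemy tag in the blackboard's enemy key, clearing it when sensing fails.
; Each tick sets the controlled character's Aiming and Shooting flags according to whether a valid focus actor exists.
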(event OnTargetPerceptionUpdated(AIPerception)
  (params (Actor :type Actor%20Object%20Reference) (Stimulus :type AI%20Stimulus%20Structure))
  (bind _blackboard_comp (Variables|Default|GetBlackBoard_Comp))
  (bind _enemykey (Variables|Default|GetEnemyKey))
  ;[1 1 1] Check whether actor has enemy tag, if they do, ignore it
  (if (not (Actor|ActorHasTag Actor "Enemy"))
    ;[1 1 1] AI Sensing the player's presence and updating / clearing the Blackboard Key
    (if (.bSuccessfullySensed (Utilities|Struct|BreakAIStimulus Stimulus))
      (AI|Components|Blackboard|SetValueasObject _blackboard_comp _enemykey Actor)
      (else
        (AI|Components|Blackboard|ClearValue _blackboard_comp _enemykey)))))

(event EventBeginPlay
  ;[1 1 1] Asset Binding
  (bind _blackboardcomponent (Class|AIController|UseBlackboard "/Game/Dynamic/Character/AI/Guard_Behaviour_Data.Guard_Behaviour_Data"))
  (Variables|Default|SetBlackBoard_Comp _blackboardcomponent)
  (AI|RunBehaviorTree "/Game/Dynamic/Character/AI/Guard_Behaviour.Guard_Behaviour"))

(event EventTick
  (params (DeltaSeconds :type Float%20%28single-precision%29))
  (bind _returnvalue (Class|AIController|GetFocusActor))
  (bind _returnvalue_2 (Utilities|IsValid _returnvalue))
  ;[1 1 1] Make the AI Aim at the player if the player is in focus
  (bind _ascharacter (Utilities|Casting|CastToCharacter (Pawn|GetControlledPawn)))
  (Variables|/Game/Dynamic/Character/Behaviour/Character.Character_C|SetAiming _ascharacter _returnvalue_2)
  (Variables|/Game/Dynamic/Character/Behaviour/Character.Character_C|SetShooting _ascharacter _returnvalue_2))

(fn ConstructionScript)