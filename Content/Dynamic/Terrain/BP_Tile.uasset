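; BP_Tile is one segment of an infinite terrain, scattering random containers, boxes, canisters, rocks and sandbag walls on BeginPlay via PlaceActors.
; Its barrier starts locked red, turns green and passable while the player overlaps LockingVolume, and relocks on exit.
; That exit also asks InfiniteTerrainGameMode to spawn the next tile, with GetAttachLocation exposing the Arrow transform as its attach point.
; Player overlap with DeleteVolume destroys the tile to save memory.
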(event OnComponentBeginOverlap(LockingVolume)
  (params (OverlappedComponent :type Primitive%20Component%20Object%20Reference) (OtherActor :type Actor%20Object%20Reference) (OtherComp :type Primitive%20Component%20Object%20Reference) (OtherBodyIndex :type Integer) (bFromSweep :type Boolean) (SweepResult :type Hit%20Result%20Structure%20%28by%20ref%29))
  (Utilities|IsPlayerActor OtherActor)
  (CallFunction|Unlock))

(event OnComponentEndOverlap(LockingVolume)
  (params (OverlappedComponent :type Primitive%20Component%20Object%20Reference) (OtherActor :type Actor%20Object%20Reference) (OtherComp :type Primitive%20Component%20Object%20Reference) (OtherBodyIndex :type Integer))
  (Utilities|IsPlayerActor OtherActor)
  (CallFunction|Lock)
  ;[1 1 1] Spawn our next tile after we exit a tile
  (bind _asinfinite_terrain_game_mode (Utilities|Casting|CastToInfiniteTerrainGameMode (Game|GetGameMode)))
  (Default|SpawnTile _asinfinite_terrain_game_mode))

(event OnComponentBeginOverlap(DeleteVolume)
  (params (OverlappedComponent :type Primitive%20Component%20Object%20Reference) (OtherActor :type Actor%20Object%20Reference) (OtherComp :type Primitive%20Component%20Object%20Reference) (OtherBodyIndex :type Integer) (bFromSweep :type Boolean) (SweepResult :type Hit%20Result%20Structure%20%28by%20ref%29))
  ;[1 1 1] If we overlap the DeleteVolume, delete the Tile (help manage memory)
  (Utilities|IsPlayerActor OtherActor)
  (Actor|DestroyActor))

(event EventBeginPlay
  (CallFunction|Lock)
  (Class|Tile|PlaceActors "/Game/Dynamic/Terrain/Props/BP_Container.BP_Container_C" 1 3)
  (Class|Tile|PlaceActors "/Game/Dynamic/Terrain/Props/BP_Container_Open.BP_Container_Open_C" 0 2)
  (Class|Tile|PlaceActors "/Game/Dynamic/Terrain/Props/BP_Box.BP_Box_C" 2 5)
  (Class|Tile|PlaceActors "/Game/Dynamic/Terrain/Props/BP_Canister.BP_Canister_C" 1 7)
  (Class|Tile|PlaceActors "/Game/Dynamic/Terrain/Props/BP_Rock01.BP_Rock01_C" 0 3)
  (Class|Tile|PlaceActors "/Game/Dynamic/Terrain/Props/BP_Rock02.BP_Rock02_C" 0 3)
  (Class|Tile|PlaceActors "/Game/Dynamic/Terrain/Props/BP_Rock03.BP_Rock03_C" 0 3)
  (Class|Tile|PlaceActors "/Game/Dynamic/Terrain/Props/BP_SandbagWall.BP_SandbagWall_C" 0 3))

(fn ConstructionScript)

(fn GetAttachLocation
  ;[1 1 1] Gets the Transform of our Arrow component (where we are attaching the next tile)
  (return (Transformation|GetWorldTransform (Variables|Default|GetArrow))))

(fn Unlock
  (bind _barrier (Variables|Default|GetBarrier))
  ;[1 1 1] "Unlock" the barrier by disabling collision, and set the barrier to green
  (Collision|SetCollisionEnabled _barrier "NoCollision")
  (Rendering|Material|SetMaterial _barrier 0 "/Game/Dynamic/Terrain/MI_Barrier_Green.MI_Barrier_Green"))

(fn Lock
  (bind _barrier (Variables|Default|GetBarrier))
  ;[1 1 1] "Lock" the barrier by re-enabling Collision, and set the barrier to red
  (Collision|SetCollisionEnabled _barrier "QueryAndPhysics")
  (Rendering|Material|SetMaterial _barrier 0 "/Game/Dynamic/Terrain/MI_Barrier_Red.MI_Barrier_Red"))