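; Tile Blueprint for infinite terrain that gates the player with a barrier and chains into newly spawned tiles.
; The barrier starts locked (red, collidable), turns green and passable while the player overlaps LockingVolume, then relocks on exit and asks InfiniteTerrainGameMode to spawn the next tile.
; GetAttachLocation exposes the Arrow's world transform as the next tile's attach point.
; Player overlap with DeleteVolume destroys the tile to manage memory.
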(event OnComponentBeginOverlap(LockingVolume)
  (params (OverlappedComponent :type Primitive%20Component%20Object%20Reference) (OtherActor :type Actor%20Object%20Reference) (OtherComp :type Primitive%20Component%20Object%20Reference) (OtherBodyIndex :type Integer) (bFromSweep :type Boolean) (SweepResult :type Hit%20Result%20Structure%20%28by%20ref%29))
  (Utilities|IsPlayerActor OtherActor)
  (CallFunction|Unlock))

(event OnComponentEndOverlap(LockingVolume)
  (params (OverlappedComponent :type Primitive%20Component%20Object%20Reference) (OtherActor :type Actor%20Object%20Reference) (OtherComp :type Primitive%20Component%20Object%20Reference) (OtherBodyIndex :type Integer))
  (Utilities|IsPlayerActor OtherActor)
  (CallFunction|Lock)
  ;[1 1 1] Spawn our next tile after we exit a tile
  (bind _asinfinite_terrain_game_mode (Utilities|Casting|CastToInfiniteTerrainGameMode (Game|GetGameMode)))
  (Default|SpawnTile _asinfinite_terrain_game_mode))

(event OnComponentBeginOverlap(DeleteVolume)
  (params (OverlappedComponent :type Primitive%20Component%20Object%20Reference) (OtherActor :type Actor%20Object%20Reference) (OtherComp :type Primitive%20Component%20Object%20Reference) (OtherBodyIndex :type Integer) (bFromSweep :type Boolean) (SweepResult :type Hit%20Result%20Structure%20%28by%20ref%29))
  ;[1 1 1] If we overlap the DeleteVolume, delete the Tile (help manage memory)
  (Utilities|IsPlayerActor OtherActor)
  (Actor|DestroyActor))

(event EventBeginPlay
  (CallFunction|Lock))

(fn ConstructionScript)

(fn GetAttachLocation
  ;[1 1 1] Gets the Transform of our Arrow component (where we are attaching the next tile)
  (return (Transformation|GetWorldTransform (Variables|Default|GetArrow))))

(fn Unlock
  (bind _barrier (Variables|Default|GetBarrier))
  ;[1 1 1] "Unlock" the barrier by disabling collision, and set the barrier to green
  (Collision|SetCollisionEnabled _barrier "NoCollision")
  (Rendering|Material|SetMaterial _barrier 0 "/Game/Dynamic/Terrain/GreenBarrier.GreenBarrier"))

(fn Lock
  (bind _barrier (Variables|Default|GetBarrier))
  ;[1 1 1] "Lock" the barrier by re-enabling Collision, and set the barrier to red
  (Collision|SetCollisionEnabled _barrier "QueryAndPhysics")
  (Rendering|Material|SetMaterial _barrier 0 "/Game/Dynamic/Terrain/RedBarrier.RedBarrier"))